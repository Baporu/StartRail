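; BP_Bullet is a projectile that flies in a straight line and destroys itself on hitting an enemy.
; Tick moves it along its forward vector by Speed scaled by delta seconds, without sweep, so contact relies on overlap events.
; Overlapping a BP_Enemy destroys the bullet, applying no damage here, while other actors are ignored.
; An explosion emitter spawn node is present but unconnected, so it never plays.
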(event `self.ReceiveActorBeginOverlap`
  (params (OtherActor :type "Actor Object Reference"))
  (cast `/Game/HSS/Blueprints/BP_Enemy` OtherActor)
  (`self.K2_DestroyActor`))

(event `self.ReceiveTick`
  (params (DeltaSeconds :type "Float (single-precision)"))
  (`self.K2_SetActorLocation` (+ (`self.K2_GetActorLocation`) (* (`self.GetActorForwardVector`) (`self.Speed`) (`GameplayStatics.GetWorldDeltaSeconds`)))))

(fn `UserConstructionScript`)