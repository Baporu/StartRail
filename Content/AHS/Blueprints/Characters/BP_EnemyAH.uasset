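; Enemy character Blueprint that holds HP, exposes it to callers and sets its overhead health bar widget once on BeginPlay.
; TakeDamage applies fixed damage for basic or skill attacks, destroying the actor at zero HP without refreshing the bar.
; A helper counts enemies of this class by incrementing EnemyNumber without a visible reset.
; Name display and extra widget creation are unwired in the event graph.
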(event `self.ReceiveBeginPlay`
  (bind _aswbp_enemy_health_bar (cast `/Game/AHS/UI/WBP_Enemy_Health_Bar` (`WidgetComponent.GetWidget` (`self.HealthBar and ToughnessBar`))))
  (`ProgressBar.SetPercent` (`/Game/AHS/UI/WBP_Enemy_Health_Bar.HealthBar` _aswbp_enemy_health_bar) (/ (`self.HP`) 100.0)))

(fn `ReturnBasicInfo`
  (returns (CurrentHP :type "Float (double-precision)"))
  (return (`self.HP`)))

(fn `ReturnCurrentEnemyNum`
  (returns (OnFieldEnemyNum :type Integer))
  (bind _outactors (`GameplayStatics.GetAllActorsOfClass` "BP_EnemyAH_C"))
  (for _ _outactors
    (set `self.EnemyNumber` (+ (`self.EnemyNumber`) 1)))
  (return (`self.EnemyNumber`)))

(fn `ShowEnemyName`
  (bind _output_get (set `self.ShownEnemyName` (`KismetTextLibrary.Conv_StringToText` (`KismetSystemLibrary.GetDisplayName` (`self.Enemy`)))))
  (`TextRenderComponent.K2_SetText` (`self.EnemyName`) _output_get)
  (`KismetSystemLibrary.PrintString` (`KismetTextLibrary.Conv_TextToString` _output_get)))

(fn `TakeDamage`
  (params (ATKType :type Name))
  (returns (UpdatedHP :type "Float (double-precision)"))
  ; 공격받은 타입이 일반공격인지, 스킬인지 판별
  (set `self.TakenATKType` ATKType)
  (if (== (`self.TakenATKType`) "BasicATK")
    ; 일반공격 계수
    (set `self.DMGAmount` 10.0)
    (else
      ; 스킬 공격 계수
      (set `self.DMGAmount` 50.0)))
  ; 데미지 계산
  (bind _output_get (set `self.HP` (- (`self.HP`) (`self.DMGAmount`))))
  (if (<= (`self.HP`) 0.0)
    ; 죽음 상태
    (`KismetSystemLibrary.PrintString` "Dead")
    (`self.K2_DestroyActor`)
    (return 0.0)
    (else
      (return _output_get))))

(fn `UserConstructionScript`)