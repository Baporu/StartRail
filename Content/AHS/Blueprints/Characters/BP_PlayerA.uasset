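; BP_PlayerA is a player character Blueprint holding HP and skill points, apparently for skill-point-based combat against BP_EnemyA.
; UpdateSkillPoints adds a point for a basic attack and spends one for any other attack type, clamped between zero and five.
; ReturnBasicInfo exposes HP and skill points, while CurrentEnemyNum counts BP_EnemyA actors by incrementing EnemyNum without a visible reset.
; BeginPlay and the construction script are empty.
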(event `self.ReceiveBeginPlay`)

(fn `CurrentEnemyNum`
  (returns (OnFieldEnemyNum :type Integer))
  (bind _outactors (`GameplayStatics.GetAllActorsOfClass` "/Game/AHS/Blueprints/Characters/BP_EnemyA.BP_EnemyA_C"))
  (for _ _outactors
    (set `self.EnemyNum` (+ (`self.EnemyNum`) 1)))
  (return (`self.EnemyNum`)))

(fn `ReturnBasicInfo`
  (returns (CurrentHP :type "Float (double-precision)") (CurrentSkillPoint :type "Float (double-precision)"))
  (return (`self.HP`) (`self.SkillPoint`)))

(fn `UpdateSkillPoints`
  (params (ATKType :type Name))
  (returns (UpdatedSkillpoints :type "Float (double-precision)"))
  (set `self.ActionType` ATKType)
  (if (== (`self.ActionType`) "BasicATK")
    ; 기본 공격 타입이면, 스킬 포인트 증가
    (if (< (`self.SkillPoint`) 5.0)
      (bind _output_get (set `self.SkillPoint` (+ (`self.SkillPoint`) 1.0)))
      (return _output_get)
      (else
        (bind _output_get_2 (set `self.SkillPoint` 5.0))
        (return _output_get_2)))
    (else
      ; 스킬 공격 타입이면, 스킬 포인트 감소
      (if (> (`self.SkillPoint`) 0.0)
        (bind _output_get_3 (set `self.SkillPoint` (- (`self.SkillPoint`) 1.0)))
        (return _output_get_3)
        (else
          (bind _output_get_4 (set `self.SkillPoint` 0.0))
          (return _output_get_4))))))

(fn `UserConstructionScript`)