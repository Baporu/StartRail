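; Player character for turn-based combat, with its own HP and skill point state.
; On BeginPlay it looks up its selected character in DT_CharInfo and, if found, takes the first invalid slot in BP_TurnGameMode's Units array.
; Basic attacks add a skill point and other attack types spend one, within fixed bounds.
; Helper functions report HP and skill points and count BP_Enemy actors in the level.
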(event `self.ReceiveBeginPlay`
  (bind _returnvalue (`|GetDataTableRow` "/Game/AHS/Blueprints/Character_Info/DT_CharInfo.DT_CharInfo" (`|GetEnumeratorName` (`self.SelectCharName`)))
    (:`then`
      (bind _output_get (set `self.CharacterName` (`|GetEnumeratorName` (`.Name_36_508548F44617662EE4BAA0A15A9233A7` (break `/Game/AHS/Blueprints/Character_Info/S_Character_BasicStats` _returnvalue)))))
      (`KismetSystemLibrary.PrintString` (`KismetStringLibrary.Conv_NameToString` _output_get))
      (`self.SetToUnits`))))

(fn `CurrentEnemyNum`
  (returns (OnFieldEnemyNum :type Integer))
  (bind _outactors (`GameplayStatics.GetAllActorsOfClass` "/Game/AHS/Blueprints/Characters/BP_Enemy.BP_Enemy_C"))
  (for _ _outactors
    (set `self.EnemyNum` (+ (`self.EnemyNum`) 1)))
  (return (`self.EnemyNum`)))

(fn `ReturnBasicInfo`
  (returns (CurrentHP :type "Float (double-precision)") (CurrentSkillPoint :type "Float (double-precision)"))
  (return (`self.HP`) (`self.SkillPoint`)))

(fn `SetToUnits`
  (bind _asbp_turn_game_mode (cast `/Game/SHS/Blueprints/BP_TurnGameMode` (`GameplayStatics.GetGameMode`)))
  (bind _units (`/Game/SHS/Blueprints/BP_TurnGameMode.Units` _asbp_turn_game_mode))
  (for (_array_element _array_index) _units
    ; foreach (unit : units)           if (!unit.isValid())             units[i] = this;
    (`/Engine/EditorBlueprintResources/StandardMacros.IsValid` _array_element
      (:`Is Not Valid`
        (`KismetArrayLibrary.Array_Set` _units _array_index self)
        (break)))))

(fn `UpdateSkillPoints`
  (params (ATKType :type Name))
  (returns (UpdatedSkillpoints :type "Float (double-precision)"))
  (set `self.ActionType` ATKType)
  (if (== (`self.ActionType`) "BasicATK")
    ; 기본 공격 타입이면, 스킬 포인트 증가
    (if (< (`self.SkillPoint`) 5.0)
      (bind _output_get (set `self.SkillPoint` (+ (`self.SkillPoint`) 1.0)))
      (return _output_get)
      (else
        (bind _output_get_2 (set `self.SkillPoint` 5.0))
        (return _output_get_2)))
    (else
      ; 스킬 공격 타입이면, 스킬 포인트 감소
      (if (> (`self.SkillPoint`) 0.0)
        (bind _output_get_3 (set `self.SkillPoint` (- (`self.SkillPoint`) 1.0)))
        (return _output_get_3)
        (else
          (bind _output_get_4 (set `self.SkillPoint` 0.0))
          (return _output_get_4))))))

(fn `UserConstructionScript`)