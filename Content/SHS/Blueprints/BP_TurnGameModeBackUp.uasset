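; Turn-based combat game mode, named as a backup, that orders characters by lowest Action Value.
; StartTurn and EndTurn both subtract the active character's value from the others.
; StartTurn also triggers enemy attacks or, in auto mode, player AutoAttack from inside the enemy loop.
; EndTurn resets the active value and calls FindActiveUnit, which picks the first character after a hand-written recursive merge sort using a scratch array.
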(event `self.ReceiveBeginPlay`
  (`KismetSystemLibrary.PrintString` "GameMode Enable" true true (struct :`G` 0.66 :`B` 1.0 :`A` 1.0) 5.0))

(event `self.ReceiveTick`
  (params (DeltaSeconds :type "Float (single-precision)"))
  (if (`self.IsAuto`)
    _))

(fn `EndTurn`
  (bind _activecharacter (`self.ActiveCharacter`))
  (bind _actionvalue (`/Game/SHS/Blueprints/BP_CharacterS.ActionValue` _activecharacter))
  ; foreach (unit : units)        if (unit.isValid() && active_unit != unit) unit.actV -= active_unit.actV;
  (for _array_element (`self.Characters`)
    (`/Engine/EditorBlueprintResources/StandardMacros.IsValid` _array_element
      (:`Is Valid`
        (if (not (== _array_element _activecharacter))
          (bind _actionvalue_2 (`/Game/SHS/Blueprints/BP_CharacterS.ActionValue` _array_element))
          (bind _output_get (set `/Game/SHS/Blueprints/BP_CharacterS.ActionValue` (- _actionvalue_2 _actionvalue) _array_element))
          (`KismetSystemLibrary.PrintString` (`KismetStringLibrary.BuildString_Int` (`KismetStringLibrary.BuildString_Int` (`KismetStringLibrary.BuildString_Int` (`KismetSystemLibrary.GetDisplayName` _array_element) ": " _actionvalue_2 " - ") "" _actionvalue " = ") "" _output_get) true true (struct :`G` 0.838542 :`B` 0.654446 :`A` 1.0) 5.0)))))
  (`/Game/SHS/Blueprints/BP_CharacterS.SetBaseAV` _activecharacter)
  (`self.FindActiveUnit`))

(fn `FindActiveUnit`
  (bind _characters (`self.Characters`))
  (bind _activecharacter (`self.ActiveCharacter`))
  (`self.SortUnits`)
  (set `self.ActiveCharacter` (`|GetArrayItem` _characters))
  (`KismetSystemLibrary.PrintString` (`KismetStringLibrary.Concat_StrStr` "Active Unit: " (`KismetSystemLibrary.GetDisplayName` _activecharacter)) true true (struct :`R` 1.0 :`G` 0.232694 :`B` 0.765948 :`A` 1.0) 20.0)
  (`KismetSystemLibrary.PrintString` (`KismetStringLibrary.BuildString_Int` "Action Value: " "" (`/Game/SHS/Blueprints/BP_CharacterS.ActionValue` _activecharacter)) true true (struct :`R` 1.0 :`G` 0.23074 :`B` 0.768151 :`A` 1.0) 20.0)
  (for (_array_element _array_index) _characters
    (`/Engine/EditorBlueprintResources/StandardMacros.IsValid` _array_element
      (:`Is Valid`
        (`KismetSystemLibrary.PrintString` (`KismetStringLibrary.Concat_StrStr` (`KismetStringLibrary.BuildString_Int` "Unit[" "" _array_index "]: ") (`KismetSystemLibrary.GetDisplayName` _array_element)) true true (struct :`G` 0.66 :`B` 1.0 :`A` 1.0) 10.0)))))

(fn `Merge`
  (params (left :type Integer) (right :type Integer))
  (locals (mid :type Integer) (i :type Integer) (j :type Integer) (k :type Integer) (temp :type Integer) (SortingArray :type "Array of /Game/SHS/Blueprints/BP_CharacterS Object Reference"))
  (bind _k (`local.k`))
  (bind _i (`local.i`))
  (bind _j (`local.j`))
  (bind _i_2 (`local.i`))
  (bind _temp (`local.temp`))
  (bind _sortingarray (`local.SortingArray`))
  (bind _k_2 (`local.k`))
  (bind _characters (`self.Characters`))
  (bind _output_get (set `local.mid` (/ (+ left right) 2)))
  (bind _output_get_2 (set `local.i` left))
  (bind _output_get_3 (set `local.j` (+ _output_get 1)))
  (set `local.k` left)
  ; while (i <= mid && j <= right)
  (while (and (<= _output_get_2 _output_get) (<= _output_get_3 right))
    ;; if (units[i].actV <= units[j].actV)                                                                        arr[k++] = units[i++];
    (if (<= (`/Game/SHS/Blueprints/BP_CharacterS.ActionValue` (`|GetArrayItem` (`self.Characters`) (`local.i`))) (`/Game/SHS/Blueprints/BP_CharacterS.ActionValue` (`|GetArrayItem` (`self.Characters`) (`local.j`))))
      (`KismetArrayLibrary.Array_Set` (`local.SortingArray`) _k (`|GetArrayItem` (`self.Characters`) _i))
      (set `local.k` (+ 1 _k))
      (set `local.i` (+ 1 _i))
      (else
        ;; else arr[k++] = units[j++]
        (`KismetArrayLibrary.Array_Set` _sortingarray _k_2 (`|GetArrayItem` _characters _j))
        (set `local.k` (+ 1 _k_2))
        (set `local.j` (+ 1 _j)))))
  ; temp = i > mid ? j : i;
  (if (> _i_2 (`local.mid`))
    (set `local.temp` (`local.j`))
    (else
      (set `local.temp` _i_2)))
  ; while (k <= right)                                                                                     arr[k++] = units[temp++];
  (while (<= (`local.k`) (`local.right`))
    (`KismetArrayLibrary.Array_Set` _sortingarray _k_2 (`|GetArrayItem` _characters _temp))
    (set `local.k` (+ 1 _k_2))
    (set `local.temp` (+ _temp 1)))
  ; for (int i = left; i <= right; i++)                 units[i] = arr[i];
  (for _index (range (`local.left`) (+ (`local.right`) 1))
    (`KismetArrayLibrary.Array_Set` _characters _index (`|GetArrayItem` _sortingarray _index))))

(fn `Partition`
  (params (left :type Integer) (right :type Integer))
  (locals (mid :type Integer))
  ; if (left < right)                     mid = (left + right) / 2
  (if (< left right)
    (bind _output_get (set `local.mid` (/ (+ left right) 2)))
    ; Partition(left, mid)        Partition(mid + 1, right)  Merge(left, right)
    (`self.Partition` left _output_get)
    (`self.Partition` (+ _output_get 1) right)
    (`self.Merge` left right)))

(fn `SortUnits`
  (locals (ArrLength :type Integer :default 0))
  (bind _arrlength (`local.ArrLength`))
  ; foreach (unit : units)             if (units != None) arrLen++;     else break;
  (for _array_element (`self.Characters`)
    (`/Engine/EditorBlueprintResources/StandardMacros.IsValid` _array_element
      (:`Is Valid`
        (set `local.ArrLength` (+ _arrlength 1)))
      (:`Is Not Valid`
        (break))))
  ; Partition(0, arrLen - 1)
  (`self.Partition` 0 (- _arrlength 1)))

(fn `StartTurn`
  (bind _activecharacter (`self.ActiveCharacter`))
  (bind _actionvalue (`/Game/SHS/Blueprints/BP_CharacterS.ActionValue` _activecharacter))
  ; foreach (unit : units)    if (unit.isValid() && active_unit != unit) unit.actV -= active_unit.actV;
  (for _array_element (`self.Characters`)
    (`/Engine/EditorBlueprintResources/StandardMacros.IsValid` _array_element
      (:`Is Valid`
        (if (!= _array_element _activecharacter)
          (bind _actionvalue_2 (`/Game/SHS/Blueprints/BP_CharacterS.ActionValue` _array_element))
          (bind _output_get (set `/Game/SHS/Blueprints/BP_CharacterS.ActionValue` (- _actionvalue_2 _actionvalue) _array_element))
          (bind _returnvalue (`KismetSystemLibrary.GetDisplayName` _array_element))
          ; 로그 남기는 용
          (`KismetSystemLibrary.PrintString` (`KismetStringLibrary.BuildString_Int` (`KismetStringLibrary.BuildString_Int` (`KismetStringLibrary.BuildString_Int` _returnvalue ": " _actionvalue_2 " - ") "" _actionvalue " = ") "" _output_get) true true (struct :`G` 0.838542 :`B` 0.654446 :`A` 1.0) 5.0)
          (else
            (`KismetSystemLibrary.PrintString` (`KismetStringLibrary.BuildString_Int` _returnvalue ": " _actionvalue " ") true true (struct :`G` 0.838542 :`B` 0.654446 :`A` 1.0) 5.0))))))
  ; foreach (enemy : enemies)     if (enemy.isValid() && active_unit == enemy) enemy.Attack();
  (for _array_element_2 (`self.EnemySs`)
    (`/Engine/EditorBlueprintResources/StandardMacros.IsValid` _array_element_2
      (:`Is Valid`
        (if (== _activecharacter _array_element_2)
          (`/Game/SHS/Blueprints/BP_CharacterS.Attack` _array_element_2)
          (else
            ; else if (isAuto)                   player.AutoAttack();
            (if (`self.IsAuto`)
              (bind _asbp_player_s (cast `/Game/SHS/Blueprints/BP_PlayerS` _activecharacter))
              (`/Game/SHS/Blueprints/BP_PlayerS.AutoAttack` _asbp_player_s)))))
      (:`Is Not Valid`
        (break)))))

(fn `UserConstructionScript`)