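; Game mode for action-value turn-based combat, where the unit with the lowest value acts next.
; Its logic merge-sorts Units to pick the active one, subtracts its value from the others, triggers enemy or auto-player attacks, then resets it.
; StartTurn, FindActiveUnit, EndTurn, SortUnits and Merge have disconnected entries, so those bodies never run.
; BeginPlay only prints, Tick does nothing, and TestSort is a logged merge sort on a test array.
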(event `self.ReceiveBeginPlay`
  (`KismetSystemLibrary.PrintString` "GameMode Enable" true true (struct :`G` 0.66 :`B` 1.0 :`A` 1.0) 5.0))

(event `self.ReceiveTick`
  (params (DeltaSeconds :type "Float (single-precision)"))
  (if (`self.IsAuto`)
    _))

(fn `EndTurn`)

(fn `FindActiveUnit`)

(fn `Merge`
  (params (left :type Integer) (right :type Integer))
  (locals (mid :type Integer) (i :type Integer) (j :type Integer) (k :type Integer) (temp :type Integer) (SortingArray :type "Array of /Game/SHS/Blueprints/BP_Character Object Reference")))

(fn `Partition`
  (params (left :type Integer) (right :type Integer))
  (locals (mid :type Integer))
  ; if (left < right)                     mid = (left + right) / 2
  (if (< left right)
    (bind _output_get (set `local.mid` (/ (+ left right) 2)))
    ; Partition(left, mid)        Partition(mid + 1, right)  Merge(left, right)
    (`self.Partition` left _output_get)
    (`self.Partition` (+ _output_get 1) right)
    (`self.Merge` left right)))

(fn `SortUnits`
  (locals (ArrLength :type Integer :default 0)))

(fn `StartTurn`)

(fn `TestSort`
  (params (left :type Integer) (right :type Integer))
  (locals (mid :type Integer) (i :type Integer) (j :type Integer) (k :type Integer) (temp :type Integer) (testArr2 :type "Array of Integer") (testStr :type String :default "Before Sort:"))
  (bind _k (`local.k`))
  (bind _i (`local.i`))
  (bind _j (`local.j`))
  (bind _i_2 (`local.i`))
  (bind _temp (`local.temp`))
  (bind _left (`local.left`))
  (bind _right (`local.right`))
  (bind _testarr2 (`local.testArr2`))
  (bind _teststr (`local.testStr`))
  (bind _teststr_2 (`local.testStr`))
  (bind _testarr (`self.testArr`))
  (bind _testarr_2 (`self.testArr`))
  (bind _k_2 (`local.k`))
  (if (< left right)
    (`KismetSystemLibrary.PrintString` (`KismetStringLibrary.BuildString_Int` "Left: " "" left))
    (`KismetSystemLibrary.PrintString` (`KismetStringLibrary.BuildString_Int` "Right: " "" right))
    (for _index (range left (+ right 1))
      (set `local.testStr` (`KismetStringLibrary.BuildString_Int` _teststr_2 " " (`|GetArrayItem` (`self.testArr`) _index))))
    (`KismetSystemLibrary.PrintString` _teststr_2 true true (struct :`R` 1.0 :`A` 1.0) 30.0)
    (bind _output_get (set `local.mid` (/ (+ left right) 2)))
    (`self.TestSort` left _output_get)
    (`self.TestSort` (+ _output_get 1) right)
    (bind _output_get_2 (set `local.mid` (/ (+ _left _right) 2)))
    (`KismetSystemLibrary.PrintString` (`KismetStringLibrary.BuildString_Int` "Mid = " "" _output_get_2))
    (bind _output_get_3 (set `local.i` _left))
    (`KismetSystemLibrary.PrintString` (`KismetStringLibrary.BuildString_Int` "i = " "" _output_get_3))
    (bind _output_get_4 (set `local.j` (+ _output_get_2 1)))
    (`KismetSystemLibrary.PrintString` (`KismetStringLibrary.BuildString_Int` "j = " "" _output_get_4))
    (bind _output_get_5 (set `local.k` _left))
    (`KismetSystemLibrary.PrintString` (`KismetStringLibrary.BuildString_Int` "k = " "" _output_get_5))
    ; while (i <= mid && j <= right)
    (while (and (<= _output_get_3 _output_get_2) (<= _output_get_4 _right))
      ;; if (units[i].actV <= units[j].actV)                                                                        arr[k++] = units[i++];
      (if (<= (`|GetArrayItem` _testarr (`local.i`)) (`|GetArrayItem` _testarr (`local.j`)))
        (`KismetArrayLibrary.Array_Set` (`local.testArr2`) _k (`|GetArrayItem` _testarr_2 _i))
        (set `local.k` (+ 1 _k))
        (set `local.i` (+ 1 _i))
        (else
          ;; else arr[k++] = units[j++]
          (`KismetArrayLibrary.Array_Set` _testarr2 _k_2 (`|GetArrayItem` _testarr_2 _j))
          (set `local.k` (+ 1 _k_2))
          (set `local.j` (+ 1 _j)))))
    ; temp = i > mid ? j : i;
    (if (> _i_2 (`local.mid`))
      (set `local.temp` (`local.j`))
      (else
        (set `local.temp` _i_2)))
    ; while (k <= right)                                                                                     arr[k++] = units[temp++];
    (while (<= (`local.k`) (`local.right`))
      (`KismetArrayLibrary.Array_Set` _testarr2 _k_2 (`|GetArrayItem` _testarr_2 _temp))
      (set `local.k` (+ 1 _k_2))
      (set `local.temp` (+ _temp 1)))
    ; for (int i = left; i <= right; i++)                 units[i] = arr[i];
    (for _index_2 (range (`local.left`) (+ (`local.right`) 1))
      (`KismetArrayLibrary.Array_Set` _testarr_2 _index_2 (`|GetArrayItem` _testarr2 _index_2)))
    (set `local.testStr` "After Sort:")
    (for _index_3 (range (`local.left`) (+ (`local.right`) 1))
      (set `local.testStr` (`KismetStringLibrary.BuildString_Int` _teststr " " (`|GetArrayItem` _testarr_2 _index_3))))
    (`KismetSystemLibrary.PrintString` _teststr true true (struct :`R` 1.0 :`A` 1.0) 30.0)))

(fn `UserConstructionScript`)