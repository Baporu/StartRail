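; Enemy unit for turn-based combat that loads data table info, shows HP, toughness and weakness icons, and picks player targets by aggro-weighted random draw.
; Attacks play a punch montage while a timeline lerps it to the target.
; Capsule overlaps apply the active player's damage, show damage numbers and end the turn.
; Weakness hits deplete toughness; breaking delays its action and removes 10% damage reduction, while death updates the game mode's units.
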(event `self.ReceiveBeginPlay`
  (bind _returnvalue_location (`KismetMathLibrary.BreakTransform` (`SceneComponent.K2_GetComponentToWorld` (`self.Attack_Location`))))
  (`Widget.SetVisibility` (`WidgetComponent.GetWidget` (`self.EnemySelection`)) "Hidden")
  (`self.ConnectTo_DataTable`)
  (`self.Init`)
  (`self.EnemyUI`)
  (set `self.E_Location` (`self.K2_GetActorLocation`))
  (set `self.E_DMG_Location` _returnvalue_location)
  (`Widget.SetVisibility` (`WidgetComponent.GetWidget` (`self.DamageNum`)) "Collapsed"))

(event `CameratoEnemy`
  ; 행동 에너미에게 카메라 타겟팅
  (`PlayerController.SetViewTargetWithBlend` (`GameplayStatics.GetPlayerController` 0) self 0.0 "VTBlend_Linear" 0.0 false))

(event `self.ReceiveActorBeginOverlap`
  (params (OtherActor :type "Actor Object Reference"))
  (`parent.ReceiveActorBeginOverlap` OtherActor))

(event `Enemy_Punch_Animation`
  ; 행동 에너미 공격 애니메이션
  (`|PlayMontage` (`self.SkeletalMesh`) "/Game/AHS/Blueprints/Animations/Exported_Animations/Punch_Anim_Montage.Punch_Anim_Montage" 1.2
    (:`then`
      ;; 이동(플레이어 -> 적 위치)
      (bind (_direction _newtrack_0) (`Timeline|EnemyToPlayer` :!via `PlayFromStart`)
        (:`Update`
          (bind _returnvalue (`KismetMathLibrary.VLerp` (`self.E_Location`) (`self.P_Location`) _newtrack_0))
          (`self.K2_SetActorLocation` _returnvalue)
          (`self.RotateToAttack` _returnvalue))))))

(event `self.Capsule.OnComponentBeginOverlap`
  (params (OverlappedComponent :type "PrimitiveComponent Object Reference") (OtherActor :type "Actor Object Reference") (OtherComp :type "PrimitiveComponent Object Reference") (OtherBodyIndex :type Integer) (bFromSweep :type Boolean) (SweepResult :type "HitResult Structure (by ref)"))
  (bind _returnvalue (`WidgetComponent.GetWidget` (`self.DamageNum`)))
  ; 타격받을 때(Capsule Collider)
  (`|PlayMontage` (`self.SkeletalMesh`) "/Game/AHS/Blueprints/Animations/Exported_Animations/Hit_Anim_Montage.Hit_Anim_Montage"
    (:`then`
      (bind _asbp_turn_game_mode (cast `/Game/HSS/Blueprints/BP_TurnGameMode` (`GameplayStatics.GetGameMode`)))
      (bind _asbp_player (cast `/Game/HSS/Blueprints/BP_Player` (`/Game/HSS/Blueprints/BP_TurnGameMode.ActiveUnit` _asbp_turn_game_mode)))
      (`self.TakeDamage` (`/Game/HSS/Blueprints/BP_Unit.Damage` _asbp_player) (`/Game/HSS/Blueprints/BP_Unit.DamageType` _asbp_player) (`/Game/HSS/Blueprints/BP_Player.AttackToughnessDamage` _asbp_player))
      ; 받은 데미지 숫자로 뜸.
      (bind _aswbp_damage_numbers (cast `/Game/AHS/UI/Enemy_UI/WBP_DamageNumbers` _returnvalue))
      (`/Game/AHS/UI/Enemy_UI/WBP_DamageNumbers.SetDamage` _aswbp_damage_numbers (`self.TakenDMG`))
      (`Widget.SetVisibility` _returnvalue "Visible")
      (`KismetSystemLibrary.Delay` 1.0)
      (`Widget.SetVisibility` _returnvalue "Collapsed")
      ; 데미지 입은 거 UI에 반영
      (`/Game/HSS/Blueprints/BP_TurnGameMode.UpdateAllEnemyUI` _asbp_turn_game_mode)
      (bind _asbp_turn_game_mode_2 (cast `/Game/HSS/Blueprints/BP_TurnGameMode` (`GameplayStatics.GetGameMode`)))
      (`/Game/HSS/Blueprints/BP_TurnGameMode.EndTurn` _asbp_turn_game_mode_2))))

(event `self.Fist.OnComponentBeginOverlap`
  (params (OverlappedComponent :type "PrimitiveComponent Object Reference") (OtherActor :type "Actor Object Reference") (OtherComp :type "PrimitiveComponent Object Reference") (OtherBodyIndex :type Integer) (bFromSweep :type Boolean) (SweepResult :type "HitResult Structure (by ref)"))
  (bind _returnvalue_location (`KismetMathLibrary.BreakTransform` (`SceneComponent.K2_GetComponentToWorld` (`self.Fist`))))
  (`GameplayStatics.SpawnEmitterAtLocation` null _returnvalue_location (struct) (0.5 0.5 0.5)))

(fn `AfterAttack`
  (bind _asbp_player (cast `/Game/HSS/Blueprints/BP_Player` (`self.AttackTargetUnit`)))
  (bind _damage (`self.CalcDamage` (`self.AttackRatio`)))
  (`/Game/HSS/Blueprints/BP_Player.TakeDamage` _asbp_player _damage (`self.DamageType`)))

(fn `Attack`
  (params (AttackTarget :type "/Game/HSS/Blueprints/BP_Unit Object Reference") (EnergyIncreasedBy :type Integer) (AttackRatio :type "Float (double-precision)"))
  (`parent.Attack` AttackTarget EnergyIncreasedBy AttackRatio)
  (`self.GetTargetPlayerLocation`)
  (`self.PrintLogAttack`)
  (`self.Enemy_Punch_Animation`))

(fn `Attack_0`
  (params (`Attack Target` :type "/Game/HSS/Blueprints/BP_Player Object Reference") (`Damage Type` :type "/Game/HSS/Blueprints/E_DamageType Enum" :default "NewEnumerator7"))
  (`KismetSystemLibrary.PrintString` (`KismetStringLibrary.Concat_StrStr` (`KismetSystemLibrary.GetDisplayName` self) "'s attack!") true true (struct :`R` 1.0 :`A` 1.0) 5.0)
  ; 애니메이션
  (set `self.P_Location` (`/Game/HSS/Blueprints/BP_Player.P_DMG_Location` `Attack Target`))
  (`self.Enemy_Punch_Animation`)
  (`/Game/HSS/Blueprints/BP_Player.TakeDamage` `Attack Target` (* (`self.AttackRatio`) (`self.BaseAttack`)) `Damage Type`))

(fn `BeforeAttack`
  (params (AttackTarget :type "/Game/HSS/Blueprints/BP_Unit Object Reference"))
  (bind _returnvalue_location (`KismetMathLibrary.BreakTransform` (`SceneComponent.K2_GetComponentToWorld` (`self.Attack_Location`))))
  (bind _output_get (set `self.AttackTargetUnit` AttackTarget))
  (bind _asbp_player (cast `/Game/HSS/Blueprints/BP_Player` _output_get))
  (set `self.P_Location` (`/Game/HSS/Blueprints/BP_Player.P_DMG_Location` _asbp_player))
  (set `self.E_Location` (`self.K2_GetActorLocation`))
  (set `self.E_DMG_Location` _returnvalue_location)
  (`self.Enemy_Punch_Animation`))

(fn `CheckDamageReduction`
  (params (DamageType :type "/Game/HSS/Blueprints/E_DamageType Enum" :default "NewEnumerator7") (ToughnessDamage :type Integer) (Damage :type Integer))
  (returns (CheckedDamage :type Integer))
  (`self.TakeToughnessDamage` DamageType ToughnessDamage)
  ; if (!isBroken)                     curHP -= damage;
  (if (`self.IsBroken`)
    (set `self.CurrentHP` (- (`self.CurrentHP`) Damage))
    (else
      ; else                 curHP -= damage * 0.9;
      (set `self.CurrentHP` (- (`self.CurrentHP`) (* Damage 0.9))))))

(fn `ConnectTo_DataTable`
  ; DT_CharInfo의 row 이름 == 설정한 CharName
  (bind _outrownames (`DataTableFunctionLibrary.GetDataTableRowNames` "/Game/AHS/Blueprints/Character_Info/DT_CharInfo.DT_CharInfo"))
  (for _array_element _outrownames
    (if (== _array_element (`KismetStringLibrary.Conv_StringToName` (`|GetEnumeratorNameAsString` (`self.EnemyCharName`))))
      (break)))
  (bind _returnvalue (`|GetDataTableRow` "/Game/AHS/Blueprints/Character_Info/DT_CharInfo.DT_CharInfo" _array_element)
    (:`then`
      (set `self.CharInfo` _returnvalue))))

(fn `EnemyUI`
  ; 기본 정보 UI 세팅(HP, 강인도)
  (bind _aswbp_enemy_health_bar (cast `/Game/AHS/UI/Enemy_UI/WBP_Enemy_Health_Bar` (`WidgetComponent.GetWidget` (`self.Widget`))))
  (`/Game/AHS/UI/Enemy_UI/WBP_Enemy_Health_Bar.Get_All_Info` _aswbp_enemy_health_bar (`self.CurrentHP`) (`self.CurrentToughness`) (`self.MaxHP`) (`self.MaxToughness`))
  (for _array_element (`self.Weaknesses`)
    (bind _outrownames (`DataTableFunctionLibrary.GetDataTableRowNames` "/Game/AHS/Blueprints/Character_Info/DT_DamageType_Info.DT_DamageType_Info"))
    (for _array_element_2 _outrownames
      (if (== _array_element_2 (`KismetStringLibrary.Conv_StringToName` (`|GetEnumeratorNameAsString` _array_element)))
        (bind _returnvalue (`|CreateWidget` "/Game/AHS/UI/Enemy_UI/WBP_Types.WBP_Types_C"))
        (bind _returnvalue_2 (`|GetDataTableRow` "/Game/AHS/Blueprints/Character_Info/DT_DamageType_Info.DT_DamageType_Info" _array_element_2)
          (:`then`
            (set `/Game/AHS/UI/Enemy_UI/WBP_Types.Image` (`.Icon_7_F662D99A42BAF4A44AE54CA5653FEEA7` (break `/Game/AHS/Blueprints/Character_Info/S_DamageType` _returnvalue_2)) _returnvalue)
            (`PanelWidget.AddChild` (`/Game/AHS/UI/Enemy_UI/WBP_Enemy_Health_Bar.TypeBox` _aswbp_enemy_health_bar) _returnvalue)
            (`UserWidget.AddToViewport` _returnvalue 0)))))))

(fn `FindAliveEnemy`
  (bind _asbp_turn_game_mode (cast `/Game/HSS/Blueprints/BP_TurnGameMode` (`GameplayStatics.GetGameMode`)))
  (for (_array_element _array_index) (`/Game/HSS/Blueprints/BP_TurnGameMode.Enemies` _asbp_turn_game_mode)
    (if (!= _array_element self)
      (`/Engine/EditorBlueprintResources/StandardMacros.IsValid` _array_element
        (:`Is Valid`
          (set `/Game/HSS/Blueprints/BP_TurnGameMode.EnemyTargetIndex` _array_index _asbp_turn_game_mode)
          (break))))))

(fn `FindTargetByAggro`
  (returns (AttackTarget :type "/Game/HSS/Blueprints/BP_Player Object Reference"))
  (locals (AggroSum :type Integer) (RandomAggro :type Integer))
  (bind _aggrosum (`local.AggroSum`))
  (bind _asbp_turn_game_mode (cast `/Game/HSS/Blueprints/BP_TurnGameMode` (`GameplayStatics.GetGameMode`)))
  (bind _players (`/Game/HSS/Blueprints/BP_TurnGameMode.Players` _asbp_turn_game_mode))
  ; foreach (player : players) if (player.isValid())                             aggroSum += player.aggro;
  (for _array_element _players
    (`/Engine/EditorBlueprintResources/StandardMacros.IsValid` _array_element
      (:`Is Valid`
        (if (not (`/Game/HSS/Blueprints/BP_Player.IsDead` _array_element))
          (bind _output_get (set `local.AggroSum` (+ _aggrosum (`/Game/HSS/Blueprints/BP_Player.Aggro` _array_element))))
          (`KismetSystemLibrary.PrintString` (`KismetStringLibrary.BuildString_Int` "Aggro Sum: " "" _output_get) false)))
      (:`Is Not Valid`
        (break))))
  (set `local.RandomAggro` (`KismetMathLibrary.RandomIntegerInRange` 1 _aggrosum))
  (bind _output_get_2 (set `local.AggroSum` 0))
  ; 플레이어 배열을 돌면서 해당 어그로 수치에 대응하는 플레이어를 찾아서 반환함 (어그로 수치만큼 배열 인덱스 = 뽑기권을 가진 셈)
  (for _array_element_2 _players
    (`/Engine/EditorBlueprintResources/StandardMacros.IsValid` _array_element_2
      (:`Is Valid`
        (if (not (`/Game/HSS/Blueprints/BP_Player.IsDead` _array_element_2))
          (bind _output_get_3 (set `local.AggroSum` (+ _output_get_2 (`/Game/HSS/Blueprints/BP_Player.Aggro` _array_element_2))))
          (if (<= (`local.RandomAggro`) _output_get_3)
            (`KismetSystemLibrary.PrintString` (`KismetStringLibrary.Concat_StrStr` "Attack Target: " (`KismetSystemLibrary.GetDisplayName` _array_element_2)) false)
            (return _array_element_2)))))))

(fn `GetTargetPlayerLocation`
  (bind _asbp_player (cast `/Game/HSS/Blueprints/BP_Player` (`self.AttackTargetUnit`)))
  (set `self.P_Location` (`/Game/HSS/Blueprints/BP_Player.P_DMG_Location` _asbp_player)))

(fn `Init`
  ;[0.15 0.15 0.15 0.5 16] 스폰되고 초기화하는 함수, Enemy의 변수 초기화 후 Unit의 변수 초기화 실행, 초기화를 마친 뒤에 Unit과 Enemy 배열에 할당됨
  (set `self.CurrentToughness` (`self.MaxToughness`))
  (set `self.IsBroken` false)
  (set `self.IsCharging` false)
  (`parent.Init`))

(fn `Setting_OriginalLocation`
  (params (TargetLocation :type "Vector Structure")))

(fn `SetToUnits`
  (bind _asbp_turn_game_mode (cast `/Game/HSS/Blueprints/BP_TurnGameMode` (`GameplayStatics.GetGameMode`)))
  (bind _units (`/Game/HSS/Blueprints/BP_TurnGameMode.Units` _asbp_turn_game_mode))
  ; foreach (unit : units)           if (!unit.isValid())             units[i] = this;
  (for (_array_element _array_index) _units
    (`/Engine/EditorBlueprintResources/StandardMacros.IsValid` _array_element
      (:`Is Not Valid`
        (`KismetArrayLibrary.Array_Set` _units _array_index self)
        (break))))
  (`self.PrintLogSet` self _array_index)
  (bind _enemies (`/Game/HSS/Blueprints/BP_TurnGameMode.Enemies` _asbp_turn_game_mode))
  ; foreach (unit : units)           if (!unit.isValid())             units[i] = this;
  (for (_array_element_2 _array_index_2) _enemies
    (`/Engine/EditorBlueprintResources/StandardMacros.IsValid` _array_element_2
      (:`Is Not Valid`
        (`KismetArrayLibrary.Array_Set` _enemies _array_index_2 self)
        (break))))
  (set `/Game/HSS/Blueprints/BP_TurnGameMode.EnemyCount` (+ (`/Game/HSS/Blueprints/BP_TurnGameMode.EnemyCount` _asbp_turn_game_mode) 1) _asbp_turn_game_mode))

(fn `StartEnemyAction`
  ; 턴 시작 시 초기화하는 함수: 약점 격파 회복, 대부분의 (디)버프들 초기화를 담당함
  (set `self.TotalTurn` (+ (`self.TotalTurn`) 1))
  (if (`self.IsBroken`)
    (set `self.IsBroken` false)
    (set `self.CurrentToughness` (`self.MaxToughness`)))
  (return))

(fn `TakeDamage`
  (params (Damage :type Integer) (DamageType :type "/Game/HSS/Blueprints/E_DamageType Enum" :default "NewEnumerator7") (ToughnessDamage :type Integer))
  (locals (IsWeakness :type Boolean))
  (bind _damage (`local.Damage`))
  (bind _returnvalue (`WidgetComponent.GetWidget` (`self.DamageNum`)))
  (bind _returnvalue_2 (* _damage 0.9))
  ; foreach (weakness : weaknesses)     if (weakness = damageType)     isWeakness = true;
  (for _array_element (`self.Weaknesses`)
    (if (`|EnumEquality` _array_element DamageType)
      (set `local.IsWeakness` true)))
  ; if (isWeakness)                             toughness -= toughnessDamage;                                        if (toughness <= 0 && !isBroken)               isBroken = true;             actionValue *= 1.25;                                                     GM.SortUnits();
  (if (`local.IsWeakness`)
    (bind _output_get (set `self.CurrentToughness` (- (`self.CurrentToughness`) (`local.ToughnessDamage`))))
    (if (and (<= _output_get 0) (not (`self.IsBroken`)))
      (set `self.IsBroken` true)
      (set `self.CurrentToughness` 0)
      (set `self.ActionValue` (* (`self.ActionValue`) 1.25))
      (bind _asbp_turn_game_mode (cast `/Game/HSS/Blueprints/BP_TurnGameMode` (`GameplayStatics.GetGameMode`)))
      (`/Game/HSS/Blueprints/BP_TurnGameMode.SortUnits` _asbp_turn_game_mode)))
  ; if (isbroken != true)                            curHP -= damage x 0.9;
  (if (!= true (`self.IsBroken`))
    (set `self.CurrentHP` (- (`self.CurrentHP`) _returnvalue_2))
    (set `self.TakenDMG` _returnvalue_2)
    (else
      ; else curHP -= damage;
      (set `self.CurrentHP` (- (`self.CurrentHP`) _damage))
      (set `self.TakenDMG` _damage)))
  ; 받은 데미지 숫자로 뜸.
  (bind _aswbp_damage_numbers (cast `/Game/AHS/UI/Enemy_UI/WBP_DamageNumbers` _returnvalue))
  (`/Game/AHS/UI/Enemy_UI/WBP_DamageNumbers.SetDamage` _aswbp_damage_numbers (`self.TakenDMG`))
  (`Widget.SetVisibility` _returnvalue "Visible")
  (bind _asbp_turn_game_mode_2 (cast `/Game/HSS/Blueprints/BP_TurnGameMode` (`GameplayStatics.GetGameMode`)))
  (`/Game/HSS/Blueprints/BP_TurnGameMode.UpdateAllEnemyUI` _asbp_turn_game_mode_2)
  ; 현재 체력이 0 이하면 사망 처리
  (if (<= (`self.CurrentHP`) 0)
    (`self.PrintLogDead`)
    (bind _asbp_turn_game_mode_3 (cast `/Game/HSS/Blueprints/BP_TurnGameMode` (`GameplayStatics.GetGameMode`)))
    (`self.FindAliveEnemy`)
    (set `/Game/HSS/Blueprints/BP_TurnGameMode.EnemyCount` (- (`/Game/HSS/Blueprints/BP_TurnGameMode.EnemyCount` _asbp_turn_game_mode_3) 1) _asbp_turn_game_mode_3)
    (`/Game/HSS/Blueprints/BP_TurnGameMode.ReorderUnits` _asbp_turn_game_mode_3 self)
    (`self.K2_DestroyActor`)))

(fn `TakeToughnessDamage`
  (params (DamageType :type "/Game/HSS/Blueprints/E_DamageType Enum" :default "NewEnumerator7") (ToughnessDamage :type Integer))
  (locals (IsWeakness :type Boolean))
  ; foreach (weakness : weaknesses)     if (weakness = damageType)     isWeakness = true;
  (for _array_element (`self.Weaknesses`)
    (if (`|EnumEquality` _array_element DamageType)
      (set `local.IsWeakness` true)))
  ; if (isWeakness)                             toughness -= toughnessDamage;                                        if (toughness <= 0 && !isBroken)               isBroken = true;             actionValue *= 1.25;                                                     GM.SortUnits();
  (if (`local.IsWeakness`)
    (bind _output_get (set `self.CurrentToughness` (- (`self.CurrentToughness`) (`local.ToughnessDamage`))))
    (if (and (<= _output_get 0) (not (`self.IsBroken`)))
      (set `self.IsBroken` true)
      (set `self.CurrentToughness` 0)
      (set `self.ActionValue` (* (`self.ActionValue`) 1.25))
      (bind _asbp_turn_game_mode (cast `/Game/HSS/Blueprints/BP_TurnGameMode` (`GameplayStatics.GetGameMode`)))
      (`/Game/HSS/Blueprints/BP_TurnGameMode.SortUnits` _asbp_turn_game_mode))))

(fn `UserConstructionScript`
  (`parent.UserConstructionScript`)
  (`SceneComponent.K2_AttachToComponent` (`self.Fist`) (`self.SkeletalMesh`) "hand_r" "KeepRelative" "KeepRelative" "KeepRelative" true))