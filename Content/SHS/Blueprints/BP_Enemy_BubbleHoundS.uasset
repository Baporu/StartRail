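; BP_Enemy_BubbleHoundS is the Bubble Hound enemy, with a single attack on its turn.
; BeginPlay sets its character name enum after the parent's initialization.
; Its StartEnemyAction override runs the parent's turn-start setup, prints a debug message, then immediately attacks the target returned by FindTargetByAggro, with no action selection.
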(event `self.ReceiveBeginPlay`
  (`parent.ReceiveBeginPlay`)
  (set `self.EnemyCharName` "NewEnumerator4"))

(fn `StartEnemyAction`
  ; 공격이 하나밖에 없으므로 턴 시작 초기화만 수행 후 바로 공격한다.
  (`parent.StartEnemyAction`)
  (`KismetSystemLibrary.PrintString` "Hound's Turn" true true (struct :`B` 1.0 :`A` 1.0) 5.0)
  (bind _attacktarget (`self.FindTargetByAggro`))
  (`self.Attack` (`self.DamageType`) _attacktarget))

(fn `UserConstructionScript`
  (`parent.UserConstructionScript`))