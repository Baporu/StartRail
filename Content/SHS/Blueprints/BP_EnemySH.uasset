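; BP_EnemySH is the enemy unit in a turn-based battle, marked as non-player on BeginPlay.
; GetDamage cuts damage by 10% until broken; weakness hits drain Toughness, and a break scales ActionValue and has BP_TurnGameModeSH re-sort units, though DamageType is unwired.
; Attack only runs FindTargetByAggro and prints a message.
; Targeting makes an aggro-weighted random roll over players, but returns when the running sum is at or below it.
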(event `self.ReceiveBeginPlay`
  (set `self.IsPlayer` false)
  (`parent.ReceiveBeginPlay`))

(fn `Attack`
  (`self.FindTargetByAggro`)
  (`KismetSystemLibrary.PrintString` "Enemy Attack!" true true (struct :`R` 0.707007 :`B` 0.90625 :`A` 1.0) 5.0))

(fn `FindTargetByAggro`
  (returns (Target :type "Object Object Reference"))
  (locals (AggroSum :type "Float (double-precision)" :default 0.0) (RandomAggro :type "Float (double-precision)"))
  (bind _aggrosum (`local.AggroSum`))
  (bind _asbp_turn_game_mode (cast `/Game/SHS/Blueprints/BP_TurnGameModeSH` (`GameplayStatics.GetGameMode`)))
  (bind (_players _players_2) (`/Game/SHS/Blueprints/BP_TurnGameModeSH.Players` _asbp_turn_game_mode))
  ; foreach (player : players) if (player.isValid())                             aggroSum += player.aggro;
  (for _array_element _players_2
    (`/Engine/EditorBlueprintResources/StandardMacros.IsValid` _array_element
      (:`Is Valid`
        (set `local.AggroSum` (+ (`local.AggroSum`) (`/Game/SHS/Blueprints/BP_EnemySH.Aggro` _array_element))))
      (:`Is Not Valid`
        (break))))
  ; aggroSum--;                randAggro = Random(0, aggroSum);                      aggroSum = 0;
  (set `local.AggroSum` (- _aggrosum 1.0))
  (set `local.RandomAggro` (* _aggrosum (`KismetMathLibrary.RandomFloat`)))
  (bind _output_get (set `local.AggroSum` 0.0))
  ; foreach (player : players)     if (player.isValid())                 aggroSum += player.aggro;                 if (randAggro <= player.aggro) return player;
  (for _array_element_2 _players_2
    (`/Engine/EditorBlueprintResources/StandardMacros.IsValid` _array_element_2
      (:`Is Valid`
        (bind _output_get_2 (set `local.AggroSum` (+ _output_get (`/Game/SHS/Blueprints/BP_EnemySH.Aggro` _array_element_2))))
        (if (<= _output_get_2 (`local.RandomAggro`))
          (return _array_element_2)))
      (:`Is Not Valid`
        (break)))))

(fn `GetDamage`
  (params (Damage :type Integer) (DamageType :type Byte :default 0) (ToughnessDamage :type Integer))
  ; if (isbroken != true)                            health -= damage x 0.9;
  (if (!= true (`self.IsBroken`))
    (set `self.Health` (- (`self.Health`) (* Damage 0.9)))
    ; foreach (weakness : weaknesses)     if (weakness = damageType)     isWeakness = true;
    (for _ (`self.Weaknesses`)
      (if (`|EnumEquality` _)
        (set `self.IsWeakness` true)))
    ; if (isWeakness)                 toughness -= toughnessDamage;                        if (toughness <= 0)               isBroken = true;                     actionValue *= 1.25;                                                                 GM.SortUnits();
    (if (`self.IsWeakness`)
      (bind _output_get (set `self.Toughness` (- (`self.Toughness`) (`local.ToughnessDamage`))))
      (if (<= _output_get 0)
        (set `self.IsBroken` true)
        (set `self.ActionValue` (* (`self.ActionValue`) 1.25))
        (bind _asbp_turn_game_mode (cast `/Game/SHS/Blueprints/BP_TurnGameModeSH` (`GameplayStatics.GetGameMode`)))
        (`/Game/SHS/Blueprints/BP_TurnGameModeSH.SortUnits` _asbp_turn_game_mode)))
    (else
      ; else health -= damage;
      (set `self.Health` (- (`self.Health`) Damage)))))

(fn `UserConstructionScript`
  (`parent.UserConstructionScript`))