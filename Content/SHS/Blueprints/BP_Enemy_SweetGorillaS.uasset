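; Turn-based elite enemy Sweet Gorilla, which normally acts twice per turn by re-entering StartEnemyAction through the FirstTurn flag.
; It attacks the aggro target to build energy, then either charges its ultimate at full energy or summons Bubble Hounds into empty enemy slots, attacking if none spawn.
; A charged ultimate replaces the next turn with repeated attacks, resets energy and blocks recharging until the summon step runs again.
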(event `self.ReceiveBeginPlay`
  (bind _returnvalue_location (`KismetMathLibrary.BreakTransform` (`SceneComponent.K2_GetComponentToWorld` (`self.Attack_Location`))))
  (`self.ConnectTo_DataTable`)
  (`self.Init`)
  (set `self.EnemyCharName` "NewEnumerator5")
  (`self.EnemyUI`)
  (set `self.E_Location` (`self.K2_GetActorLocation`))
  (set `self.E_DMG_Location` _returnvalue_location))

(fn `Attack`
  (params (DamageType :type "/Game/HSS/Blueprints/E_DamageType Enum" :default "NewEnumerator7") (AttackTarget :type "/Game/HSS/Blueprints/BP_Player Object Reference"))
  (bind _maxenergy (`self.MaxEnergy`))
  (`parent.Attack` DamageType AttackTarget)
  (bind _output_get (set `self.CurrentEnergy` (+ (`self.CurrentEnergy`) 10)))
  (if (> _output_get _maxenergy)
    (set `self.CurrentEnergy` _maxenergy)))

(fn `Init`
  (set `self.FirstTurn` true)
  (set `self.CanUseUlt` false)
  (`parent.Init`))

(fn `StartEnemyAction`
  ; 엘리트는 한 턴에 2번 행동하므로 턴 시작 초기화는 1번만 진행한다.
  (if (`self.FirstTurn`)
    (`parent.StartEnemyAction`)
    (`KismetSystemLibrary.PrintString` "Gorilla's Turn 1" true true (struct :`B` 1.0 :`A` 1.0) 5.0)
    ; 궁극기를 준비하고 있었으면 궁극기를 사용한 후 바로 턴을 마친다.
    (if (`self.IsCharging`)
      (`self.UseUltimate`)
      (set `self.CanUseUlt` false)
      (else
        ; 궁극기를 쓰지 않을 때에는 공격 - 스킬 순으로 행동하니 공격 후 행동을 다시 진행한다.
        (bind _attacktarget (`self.FindTargetByAggro`))
        (`self.Attack` (`self.DamageType`) _attacktarget)
        (set `self.FirstTurn` false)
        (`self.StartEnemyAction`)))
    (else
      ; 궁극기를 사용할 에너지가 있고, 궁극기를 사용할 수 있으면(= 전 턴에 궁극기를 쓰지 않았으면) 궁극기를 쓰고, 그렇지 않으면 소환을 실행한다.
      (`KismetSystemLibrary.PrintString` "Gorilla's Turn 2" true true (struct :`B` 1.0 :`A` 1.0) 5.0)
      (if (`self.CanUseUlt`)
        (if (== (`self.CurrentEnergy`) (`self.MaxEnergy`))
          (`self.UseUltimate`)
          (else
            (`self.SummonEnemies` :!label _label)
            (set `self.CanUseUlt` true)))
        (else
          (goto _label)))
      (set `self.FirstTurn` true))))

(fn `SummonEnemies`
  (locals (SummonCount :type Integer :default 2))
  (bind _summoncount (`local.SummonCount`))
  (bind _asbp_turn_game_mode (cast `/Game/HSS/Blueprints/BP_TurnGameMode` (`GameplayStatics.GetGameMode`)))
  ; 적 배열에 None이 있다 = 소환할 자리가 있다
  (for (_array_element _array_index) (`/Game/HSS/Blueprints/BP_TurnGameMode.Enemies` _asbp_turn_game_mode)
    (`/Engine/EditorBlueprintResources/StandardMacros.IsValid` _array_element
      (:`Is Not Valid`
        ; 소환 횟수가 남아있으면 유닛을 소환하고 횟수를 1 차감한다.
        (if (> _summoncount 0)
          (bind _spawntransform (`/Game/SHS/Blueprints/BP_EnemySpawner.GetSpawnTransform` (`/Game/HSS/Blueprints/BP_TurnGameMode.EnemySpawner` _asbp_turn_game_mode) _array_index))
          (`|SpawnActorFromClass` "/Game/HSS/Blueprints/BP_Enemy_BubbleHound.BP_Enemy_BubbleHound_C" _spawntransform "Undefined" "MultiplyWithRoot" null null)
          (bind _output_get (set `local.SummonCount` (- _summoncount 1)))
          ; 지정 횟수만큼 소환했다면 루프를 벗어난다.
          (if (== _output_get 0)
            (break))))))
  ; 자리가 없어 소환을 못 했다면 기본 공격을 수행한다.
  (if (== _summoncount 2)
    (`self.Attack` (`self.DamageType`))
    (else
      ; 소환을 했다면 위치를 다시 정렬한다.
      (`/Game/HSS/Blueprints/BP_TurnGameMode.RearrangeEnemies` _asbp_turn_game_mode))))

(fn `UserConstructionScript`
  (`parent.UserConstructionScript`))

(fn `UseUltimate`
  (if (`self.IsCharging`)
    (set `self.IsCharging` false)
    (`KismetSystemLibrary.PrintString` "Gorilla uses the ultimate!")
    (bind _attacktarget (`self.FindTargetByAggro`))
    (for _ (range 4)
      (`self.Attack` (`self.DamageType`) _attacktarget))
    (set `self.CurrentEnergy` 0)
    (else
      (set `self.IsCharging` true)
      (`KismetSystemLibrary.PrintString` "Gorilla is charging.." true true (struct :`G` 0.66 :`B` 1.0 :`A` 1.0) 20.0))))