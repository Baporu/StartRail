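; BP_Character_DanHeng is the Dan Heng character Blueprint, which casts itself to BP_Character at startup.
; On BeginPlay it runs the parent logic, reads the DanHeng row from the DT_CharInfo data table and prints that row's Name enum as a debug string.
; Tick and overlap events are disabled, and the construction script only calls the parent.
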(event `self.ReceiveBeginPlay`
  (`parent.ReceiveBeginPlay`)
  (cast `/Game/SHS/Blueprints/BP_Character` self)
  (bind _returnvalue (`|GetDataTableRow` "/Game/AHS/Blueprints/Character_Info/DT_CharInfo.DT_CharInfo" "DanHeng")
    (:`then`
      (`KismetSystemLibrary.PrintString` (`|GetEnumeratorNameAsString` (`.Name_36_508548F44617662EE4BAA0A15A9233A7` (break `/Game/AHS/Blueprints/Character_Info/S_Character_BasicStats` _returnvalue)))))))

(fn `UserConstructionScript`
  (`parent.UserConstructionScript`))