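; BP_CharacterSH is a character unit for a turn-based game, with a speed-derived action value.
; On BeginPlay it computes ActionValue as 10000 / Speed and prints it.
; SetToUnits and Attack are empty; their unit-registration and debug-print logic is disconnected.
; ReturnAV returns Speed rather than ActionValue, and ReturnName reads the name enum from DT_CharInfo's Default row.
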(event `self.ReceiveBeginPlay`
  (`self.SetBaseAV`)
  (`self.SetToUnits`))

(fn `Attack`)

(fn `ReturnAV`
  (returns (AV :type Integer))
  (return (`self.Speed`)))

(fn `ReturnName`
  (returns (ReturnName :type String))
  (bind _returnvalue (`|GetDataTableRow` "/Game/AHS/Blueprints/Character_Info/DT_CharInfo.DT_CharInfo" "Default")
    (:`then`
      (set `self.CharacterName` (`|GetEnumeratorNameAsString` (`.Name_36_508548F44617662EE4BAA0A15A9233A7` (break `/Game/AHS/Blueprints/Character_Info/S_Character_BasicStats` _returnvalue))))
      (return (`self.CharacterName`)))))

(fn `SetBaseAV`
  ; actV = 10000 / speed;
  (bind _output_get (set `self.ActionValue` (/ 10000 (`self.Speed`))))
  (`KismetSystemLibrary.PrintString` (`KismetStringLibrary.BuildString_Int` (`KismetStringLibrary.Concat_StrStr` (`KismetSystemLibrary.GetDisplayName` self) ": Set Base AV: ") "" _output_get) true true (struct :`G` 0.66 :`B` 1.0 :`A` 1.0) 1.0))

(fn `SetToUnits`)

(fn `UserConstructionScript`)