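; BP_CharacterS is a character unit for a turn-based combat system that orders actions by Action Value.
; On BeginPlay it derives its base Action Value as 10000 divided by Speed, then registers itself with BP_TurnGameMode.
; Registration fills the first invalid slot in the game mode's pre-sized Characters array.
; Attack is a print-only placeholder, and the setup steps log their results with debug prints.
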(event `self.ReceiveBeginPlay`
  (`self.SetBaseAV`)
  (`self.SetToUnits`))

(fn `Attack`
  (`KismetSystemLibrary.PrintString` "Character Attack!" true true (struct :`G` 0.66 :`B` 1.0 :`A` 1.0) 5.0))

(fn `SetBaseAV`
  ; actV = 10000 / speed;
  (bind _output_get (set `self.ActionValue` (/ 10000 (`self.Speed`))))
  (`KismetSystemLibrary.PrintString` (`KismetStringLibrary.BuildString_Int` (`KismetStringLibrary.Concat_StrStr` (`KismetSystemLibrary.GetDisplayName` self) ": Set Base AV: ") "" _output_get) true true (struct :`G` 0.66 :`B` 1.0 :`A` 1.0) 5.0))

(fn `SetToUnits`
  (bind _asbp_turn_game_mode (cast `/Game/HSS/Blueprints/BP_TurnGameMode` (`GameplayStatics.GetGameMode`)))
  (bind _characters (`/Game/HSS/Blueprints/BP_TurnGameMode.Characters` _asbp_turn_game_mode))
  ; foreach (unit : units)           if (!unit.isValid())             units[i] = this;
  (for (_array_element _array_index) _characters
    (`/Engine/EditorBlueprintResources/StandardMacros.IsValid` _array_element
      (:`Is Valid`
        (`KismetSystemLibrary.PrintString` (`KismetStringLibrary.Concat_StrStr` (`KismetStringLibrary.BuildString_Int` "Unit[" "" _array_index "] has ") (`KismetSystemLibrary.GetDisplayName` (`|GetArrayItem` _characters _array_index))) true true (struct :`G` 0.839216 :`B` 0.654902 :`A` 1.0) 5.0))
      (:`Is Not Valid`
        (`KismetArrayLibrary.Array_Set` _characters _array_index self)
        (break))))
  (`KismetSystemLibrary.PrintString` (`KismetStringLibrary.BuildString_Int` (`KismetSystemLibrary.GetDisplayName` self) " is set to units[" _array_index "]") true true (struct :`G` 0.66 :`B` 1.0 :`A` 1.0) 5.0))

(fn `UserConstructionScript`)