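; Enemy spawner for the turn-based battle that registers itself with BP_TurnGameMode on BeginPlay and holds three preset BubbleHound and SweetGorilla encounters.
; Each preset spawns its enemies, then calls the game mode's RearrangeEnemies.
; GetSpawnTransform alternates positions either side of the spawner by EnemyDistance, adjusting for odd or even EnemyCount.
; The preset selector is a constant 0, matching no preset, so nothing spawns as wired.
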(event `self.ReceiveBeginPlay`
  (bind _asbp_turn_game_mode (cast `/Game/HSS/Blueprints/BP_TurnGameMode` (`GameplayStatics.GetGameMode`)))
  (set `/Game/HSS/Blueprints/BP_TurnGameMode.EnemySpawner` self _asbp_turn_game_mode)
  (switch `int` 0
    (:`1`
      (bind _spawntransform (`self.GetSpawnTransform` 0))
      (`|SpawnActorFromClass` "/Game/HSS/Blueprints/BP_Enemy_BubbleHound.BP_Enemy_BubbleHound_C" _spawntransform "Undefined" "MultiplyWithRoot" null null)
      (bind _spawntransform_2 (`self.GetSpawnTransform` 1))
      (`|SpawnActorFromClass` "/Game/HSS/Blueprints/BP_Enemy_BubbleHound.BP_Enemy_BubbleHound_C" _spawntransform_2 "Undefined" "MultiplyWithRoot" null null)
      (bind _spawntransform_3 (`self.GetSpawnTransform` 2))
      (`|SpawnActorFromClass` "/Game/HSS/Blueprints/BP_Enemy_BubbleHound.BP_Enemy_BubbleHound_C" _spawntransform_3 "Undefined" "MultiplyWithRoot" null null))
    (:`2`
      (bind _spawntransform_4 (`self.GetSpawnTransform` 0))
      (`|SpawnActorFromClass` "/Game/HSS/Blueprints/BP_Enemy_SweetGorilla.BP_Enemy_SweetGorilla_C" _spawntransform_4 "Undefined" "MultiplyWithRoot" null null))
    (:`3`
      (bind _spawntransform_5 (`self.GetSpawnTransform` 0))
      (`|SpawnActorFromClass` "/Game/HSS/Blueprints/BP_Enemy_SweetGorilla.BP_Enemy_SweetGorilla_C" _spawntransform_5 "Undefined" "MultiplyWithRoot" null null)
      (bind _spawntransform_6 (`self.GetSpawnTransform` 1))
      (`|SpawnActorFromClass` "/Game/HSS/Blueprints/BP_Enemy_BubbleHound.BP_Enemy_BubbleHound_C" _spawntransform_6 "Undefined" "MultiplyWithRoot" null null)
      (bind _spawntransform_7 (`self.GetSpawnTransform` 2))
      (`|SpawnActorFromClass` "/Game/HSS/Blueprints/BP_Enemy_BubbleHound.BP_Enemy_BubbleHound_C" _spawntransform_7 "Undefined" "MultiplyWithRoot" null null)))
  (`/Game/HSS/Blueprints/BP_TurnGameMode.RearrangeEnemies` _asbp_turn_game_mode))

(fn `GetSpawnTransform`
  (params (EnemyIndex :type Integer))
  (returns (SpawnTransform :type "Transform Structure"))
  (locals (VectorY :type Integer))
  (bind _returnvalue (`self.GetTransform`))
  (bind _enemydistance (`self.EnemyDistance`))
  (bind _returnvalue_2 (!= (mod EnemyIndex 2) 0))
  (bind _asbp_turn_game_mode (cast `/Game/HSS/Blueprints/BP_TurnGameMode` (`GameplayStatics.GetGameMode`)))
  ; 적이 짝수일 때는 반대로 index가 홀수일 때 index * (-1), 짝수일 때는 (index + 1)을 거리에 곱해 떨어질 거리를 구할 수 있다.
  (if (!= (mod (`/Game/HSS/Blueprints/BP_TurnGameMode.EnemyCount` _asbp_turn_game_mode) 2) 0)
    (if _returnvalue_2
      (return (`KismetMathLibrary.MakeTransform` (`KismetMathLibrary.TransformLocation` _returnvalue (* (* (+ EnemyIndex 1) -1) _enemydistance))))
      (else
        (return (`KismetMathLibrary.MakeTransform` (`KismetMathLibrary.TransformLocation` _returnvalue (* _enemydistance EnemyIndex))))))
    (elif _returnvalue_2
      (return (`KismetMathLibrary.MakeTransform` (`KismetMathLibrary.TransformLocation` _returnvalue (* _enemydistance (* EnemyIndex -1)))))
      (else
        (return (`KismetMathLibrary.MakeTransform` (`KismetMathLibrary.TransformLocation` _returnvalue (* _enemydistance (+ EnemyIndex 1)))))))))

(fn `UserConstructionScript`)