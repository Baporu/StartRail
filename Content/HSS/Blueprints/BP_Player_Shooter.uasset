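; BP_Player_Shooter is the shooter player unit in a turn-based battle, built on a parent class that supplies the skill logic.
; AttackAnimation starts a montage and spawns BP_Bullet at SpawnPoint, while two other events play the idle-attack transition montages.
; Capsule overlaps count as hits only when this unit is not BP_TurnGameMode's ActiveUnit, triggering a montage, a player UI refresh and an explosion effect.
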(event `self.ReceiveBeginPlay`
  (set `self.PlayerCharName` "NewEnumerator3")
  (`parent.ReceiveBeginPlay`))

(event `self.Attack_Animation`
  (`|PlayMontage` (`self.SkeletalMesh`)
    (:`then`
      (`|SpawnActorFromClass` "/Game/AHS/Assets/Throwable_Objects/BP_Bullet.BP_Bullet_C" (`SceneComponent.K2_GetComponentToWorld` (`self.SpawnPoint`)) "Undefined" "MultiplyWithRoot" null null))))

(event `self.Capsule.OnComponentBeginOverlap`
  (params (OverlappedComponent :type "PrimitiveComponent Object Reference") (OtherActor :type "Actor Object Reference") (OtherComp :type "PrimitiveComponent Object Reference") (OtherBodyIndex :type Integer) (bFromSweep :type Boolean) (SweepResult :type "HitResult Structure (by ref)"))
  (bind _returnvalue_location (`KismetMathLibrary.BreakTransform` (`SceneComponent.K2_GetComponentToWorld` (`self.Capsule`))))
  ; 타격 애니메이션 처리
  ;; 본인 턴이 아닐 때, 상대방(적)이 공격했을 때에만 피격 처리를 함.
  (bind _asbp_turn_game_mode (cast `/Game/HSS/Blueprints/BP_TurnGameMode` (`GameplayStatics.GetGameMode`)))
  (if (!= (`/Game/HSS/Blueprints/BP_TurnGameMode.ActiveUnit` _asbp_turn_game_mode) self)
    ;; 데미지를 받았을 때
    (`|PlayMontage` (`self.SkeletalMesh`)
      (:`then`
        (bind _asbp_turn_game_mode_2 (cast `/Game/HSS/Blueprints/BP_TurnGameMode` (`GameplayStatics.GetGameMode`)))
        (`/Game/HSS/Blueprints/BP_TurnGameMode.UpdateAllPlayerUI` _asbp_turn_game_mode_2)
        (`GameplayStatics.SpawnEmitterAtLocation` "/Game/StarterContent/Particles/P_Explosion.P_Explosion" _returnvalue_location (struct) (0.5 0.5 0.5))))))

(event `self.IdletoAttack`
  (`|PlayMontage` (`self.SkeletalMesh`)))

(event `self.AttacktoIdle`
  (`|PlayMontage` (`self.SkeletalMesh`)))

(fn `Skill`
  (params (SkillTarget :type "/Game/HSS/Blueprints/BP_Unit Object Reference"))
  (`parent.Skill` SkillTarget))

(fn `UserConstructionScript`
  (`parent.UserConstructionScript`))