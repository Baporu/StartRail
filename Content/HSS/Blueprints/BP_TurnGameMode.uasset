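; Turn-based battle game mode that creates the battle UI and orders player and enemy turns by action value.
; A hand-written merge sort orders Units, and the first non-dead unit takes the turn, subtracting its action value from the others.
; Enemies act automatically; EndTurn resets the value, picks the next unit, refreshes UI and camera, then starts the delayed turn.
; Check_EnemyUnits pauses the game and shows the end-of-battle screen when no enemies remain.
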(event `self.ReceiveBeginPlay`
  ; 전체 UI 설정.
  (bind _returnvalue (`|CreateWidget` "/Game/HSS/UI/WBP_BattleWidget.WBP_BattleWidget_C"))
  (`UserWidget.AddToViewport` _returnvalue 0)
  (bind _returnvalue_2 (`|CreateWidget` "/Game/AHS/UI/WBP_Battle_ALL.WBP_Battle_ALL_C"))
  (`UserWidget.AddToViewport` _returnvalue_2 0)
  (`KismetSystemLibrary.Delay` 3.0)
  (`self.FindActiveUnit`)
  (`self.StartTurn`))

(event `self.ReceiveTick`
  (params (DeltaSeconds :type "Float (single-precision)")))

(event `Check_EnemyUnits`
  (set `self.EnemyNum` 0)
  (bind _outactors (`GameplayStatics.GetAllActorsOfClass` "/Game/HSS/Blueprints/BP_Enemy.BP_Enemy_C"))
  (for _ _outactors
    (set `self.EnemyNum` (+ (`self.EnemyNum`) 1)))
  (`KismetSystemLibrary.PrintString` (`KismetStringLibrary.Conv_IntToString` (`self.EnemyNum`)) true true (struct :`G` 1.0 :`B` 0.284882 :`A` 1.0) 500.0)
  (if (<= (`self.EnemyNum`) 0)
    ; UI 없애기
    (`GameplayStatics.SetGamePaused` true)
    (bind _foundwidgets (`WidgetBlueprintLibrary.GetAllWidgetsOfClass` "/Game/AHS/UI/WBP_Battle_TurnUI.WBP_Battle_TurnUI_C"))
    (for _array_element _foundwidgets
      (`Widget.SetVisibility` _array_element "Hidden")
      (bind _foundwidgets_2 (`WidgetBlueprintLibrary.GetAllWidgetsOfClass` "/Game/AHS/UI/WBP_PlayerParty_UI.WBP_PlayerParty_UI_C"))
      (for _array_element_2 _foundwidgets_2
        (`Widget.SetVisibility` _array_element_2 "Hidden")
        (bind _foundwidgets_3 (`WidgetBlueprintLibrary.GetAllWidgetsOfClass` "/Game/HSS/UI/WBP_BattleWidget.WBP_BattleWidget_C"))
        (for _array_element_3 _foundwidgets_3
          (`Widget.SetVisibility` _array_element_3 "Hidden")
          (bind _returnvalue (`|CreateWidget` "/Game/AHS/UI/WBP_EndofBattle.WBP_EndofBattle_C"))
          (`UserWidget.AddToViewport` _returnvalue 0))))))

(event `TimerEvent_forCamera`
  (`self.DelayTime_forCamera`))

(event `TimerEvent`
  (`self.DelayTurn`))

(fn `EndTurn`
  ; 턴을 마친 유닛의 행동 게이지를 초기화하고, 다음 턴을 가질 유닛을 찾고 턴을 시작한다.
  (`/Game/HSS/Blueprints/BP_Unit.SetBaseActionValue` (`self.ActiveUnit`))
  (`self.FindActiveUnit`)
  (`self.UpdateAllPlayerUI`)
  (`self.UpdateTurnUI`)
  (`self.UpdateCamera`)
  (`self.TimerEvent`))

(fn `FindActiveUnit`
  (bind _units (`self.Units`))
  ; 행동 게이지 적은 순으로 유닛 배열 정렬 후, 배열을 돌며 죽은 플레이어인지 확인한다. 살아있는 플레이어거나 적일 경우 턴을 가질 수 있으므로 현재 턴을 가진 유닛으로 지정한다.
  (`self.SortUnits`)
  (for _index (range (+ (`KismetArrayLibrary.Array_LastIndex` _units) 1))
    (bind _output (`|GetArrayItem` _units _index))
    (bind _asbp_player (cast `/Game/HSS/Blueprints/BP_Player` _output)
      (:`then`
        (if (not (`/Game/HSS/Blueprints/BP_Player.IsDead` _asbp_player))
          (set `self.ActiveUnit` _output :!label _label)
          (break)))
      (:`CastFailed`
        (goto _label))))
  (`KismetSystemLibrary.PrintString` "Active Unit Found"))

(fn `Merge`
  (params (left :type Integer) (right :type Integer))
  (locals (mid :type Integer) (i :type Integer) (j :type Integer) (k :type Integer) (temp :type Integer) (SortingArray :type "Array of /Game/HSS/Blueprints/BP_Unit Object Reference"))
  (bind _left (`local.left`))
  (bind _k (`local.k`))
  (bind _i (`local.i`))
  (bind _j (`local.j`))
  (bind _i_2 (`local.i`))
  (bind _temp (`local.temp`))
  (bind _units (`self.Units`))
  (bind _sortingarray (`local.SortingArray`))
  (bind _k_2 (`local.k`))
  (set `local.SortingArray` (`self.Units`))
  ; mid = (left + right) / 2
  (bind _output_get (set `local.mid` (/ (+ left right) 2)))
  ; i = left;                     j = mid + 1;             k = left;
  (bind _output_get_2 (set `local.i` _left))
  (bind _output_get_3 (set `local.j` (+ _output_get 1)))
  (set `local.k` _left)
  ; while (i <= mid && j <= right)
  (while (and (<= _output_get_2 _output_get) (<= _output_get_3 (`local.right`)))
    ;; if (units[i].actV <= units[j].actV)                                                                        arr[k++] = units[i++];
    (if (<= (`/Game/HSS/Blueprints/BP_Unit.ActionValue` (`|GetArrayItem` (`self.Units`) (`local.i`))) (`/Game/HSS/Blueprints/BP_Unit.ActionValue` (`|GetArrayItem` (`self.Units`) (`local.j`))))
      (`KismetArrayLibrary.Array_Set` (`local.SortingArray`) _k (`|GetArrayItem` (`self.Units`) _i) true)
      (set `local.k` (+ 1 _k))
      (set `local.i` (+ 1 _i))
      (else
        ;; else arr[k++] = units[j++]
        (`KismetArrayLibrary.Array_Set` _sortingarray _k_2 (`|GetArrayItem` _units _j) true)
        (set `local.k` (+ 1 _k_2))
        (set `local.j` (+ 1 _j)))))
  ; temp = i > mid ? j : i;
  (if (> _i_2 (`local.mid`))
    (set `local.temp` (`local.j`))
    (else
      (set `local.temp` _i_2)))
  ; while (k <= right)                                                                                     arr[k++] = units[temp++];
  (while (<= (`local.k`) (`local.right`))
    (`KismetArrayLibrary.Array_Set` _sortingarray _k_2 (`|GetArrayItem` _units _temp))
    (set `local.k` (+ 1 _k_2))
    (set `local.temp` (+ _temp 1)))
  ; for (int i = left; i <= right; i++)                 units[i] = arr[i];
  (for _index (range (`local.left`) (+ (`local.right`) 1))
    (`KismetArrayLibrary.Array_Set` _units _index (`|GetArrayItem` _sortingarray _index))))

(fn `Partition`
  (params (left :type Integer) (right :type Integer))
  (locals (mid :type Integer))
  (bind _left (`local.left`))
  (bind _right (`local.right`))
  ; if (left < right)                     mid = (left + right) / 2
  (if (< left right)
    (bind _output_get (set `local.mid` (/ (+ left right) 2)))
    ; Partition(left, mid)        Partition(mid + 1, right)  Merge(left, right)
    (`self.Partition` _left _output_get)
    (`self.Partition` (+ _output_get 1) _right)
    (`self.Merge` _left _right)))

(fn `ReorderUnits`
  (params (EnemyUnit :type "/Game/HSS/Blueprints/BP_Unit Object Reference"))
  (bind _units (`self.Units`))
  (`KismetArrayLibrary.Array_RemoveItem` _units EnemyUnit)
  (`KismetArrayLibrary.Array_Resize` _units 9)
  (`KismetSystemLibrary.PrintString` "Reorder Finished"))

(fn `SortUnits`
  (locals (ArrLength :type Integer :default 0))
  (bind _units (`self.Units`))
  (bind _arrlength (`local.ArrLength`))
  ; foreach (unit : units)             if (units != None) arrLen++;     else break;
  (for _array_element _units
    (`/Engine/EditorBlueprintResources/StandardMacros.IsValid` _array_element
      (:`Is Valid`
        (set `local.ArrLength` (+ _arrlength 1)))
      (:`Is Not Valid`
        (break))))
  ; Partition(0, arrLen - 1)
  (`self.Partition` 0 (- _arrlength 1))
  (for (_array_element_2 _array_index) _units
    (`/Engine/EditorBlueprintResources/StandardMacros.IsValid` _array_element_2
      (:`Is Valid`
        (`KismetSystemLibrary.PrintString` (`KismetStringLibrary.Concat_StrStr` (`KismetStringLibrary.BuildString_Int` "Unit" "[" _array_index "] = ") (`KismetSystemLibrary.GetDisplayName` _array_element_2)) true true (struct :`G` 0.66 :`B` 1.0 :`A` 1.0) 5.0))
      (:`Is Not Valid`
        (break)))))

(fn `StartTurn`
  (bind _activeunit (`self.ActiveUnit`))
  (`self.TimerEvent_forCamera`)
  ; foreach (unit : units)    if (unit.isValid() && active_unit != unit) unit.actV -= active_unit.actV;
  (for _array_element (`self.Units`)
    (`/Engine/EditorBlueprintResources/StandardMacros.IsValid` _array_element
      (:`Is Valid`
        (if (!= _array_element _activeunit)
          (bind _output_get (set `/Game/HSS/Blueprints/BP_Unit.ActionValue` (- (`/Game/HSS/Blueprints/BP_Unit.ActionValue` _array_element) (`/Game/HSS/Blueprints/BP_Unit.ActionValue` _activeunit)) _array_element))
          (`KismetSystemLibrary.PrintString` (`KismetStringLibrary.BuildString_Int` (`KismetSystemLibrary.GetDisplayName` _array_element) "'s Action Value: " _output_get))
          (if (< _output_get 0)
            (set `/Game/HSS/Blueprints/BP_Unit.ActionValue` 0 _array_element))))))
  (set `/Game/HSS/Blueprints/BP_Unit.ActionValue` 0 _activeunit)
  ; foreach (enemy : enemies)     if (enemy.isValid() && active_unit == enemy) enemy.Attack();
  (for _array_element_2 (`self.Enemies`)
    (`/Engine/EditorBlueprintResources/StandardMacros.IsValid` _array_element_2
      (:`Is Valid`
        (if (== _activeunit _array_element_2)
          (`/Game/HSS/Blueprints/BP_Enemy.StartEnemyAction` _array_element_2)
          (`self.EndTurn`)
          (else
            ; else if (isAuto)                   player.AutoAttack();
            (if (`self.IsAuto`)
              (`KismetSystemLibrary.PrintString` "player auto attack")
              (`self.EndTurn`))))))))

(fn `UpdateAllPlayerUI`
  (bind _outactors (`GameplayStatics.GetAllActorsOfClass` "/Game/HSS/Blueprints/BP_Player.BP_Player_C"))
  (for _array_element _outactors
    ; Comment
    (bind _foundwidgets (`WidgetBlueprintLibrary.GetAllWidgetsOfClass` "/Game/AHS/UI/WBP_PlayerParty_UI.WBP_PlayerParty_UI_C"))
    (for _array_element_2 _foundwidgets
      (bind _aswbp_player_party_ui (cast `/Game/AHS/UI/WBP_PlayerParty_UI` _array_element_2))
      (`/Game/AHS/UI/WBP_PlayerParty_UI.Update_PlayerPartyUI` _aswbp_player_party_ui _array_element))))

(fn `UpdateCamera`
  (bind _asbp_player (cast `/Game/HSS/Blueprints/BP_Player` (`self.ActiveUnit`))
    (:`then`
      (`/Game/HSS/Blueprints/BP_Player.SetCameratoPlayer` _asbp_player))
    (:`CastFailed`
      (bind _asbp_enemy (cast `/Game/HSS/Blueprints/BP_Enemy` (`self.ActiveUnit`)))
      (`/Game/HSS/Blueprints/BP_Enemy.CameratoEnemy` _asbp_enemy))))

(fn `UpdateTurnUI`
  (bind _foundwidgets (`WidgetBlueprintLibrary.GetAllWidgetsOfClass` "/Game/AHS/UI/WBP_Battle_TurnUI.WBP_Battle_TurnUI_C" false))
  (for _array_element _foundwidgets
    (bind _aswbp_battle_turn_ui (cast `/Game/AHS/UI/WBP_Battle_TurnUI` _array_element))
    (`/Game/AHS/UI/WBP_Battle_TurnUI.SortingBySpeed` _aswbp_battle_turn_ui)
    (`/Game/AHS/UI/WBP_Battle_TurnUI.Update_Turn` _aswbp_battle_turn_ui)))

(fn `UserConstructionScript`)