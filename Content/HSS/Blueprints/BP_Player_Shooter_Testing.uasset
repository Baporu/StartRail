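; Test player shooter Blueprint that fires bullets and overrides a parent Skill function.
; AttackAnimation plays a gun-shoot montage on the skeletal mesh and spawns BP_Bullet at the SpawnPoint transform.
; Skill skips the parent implementation and calls SetViewTargetWithBlend on the first player controller, with its Target input and the new view target left unwired.
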(event `self.Attack_Animation`
  (`|PlayMontage` (`self.SkeletalMesh`) "/Game/AHS/Assets/Mixamo_Animations/Gun/GunShoot_AnimMontage.GunShoot_AnimMontage"
    (:`then`
      (`|SpawnActorFromClass` "/Game/AHS/Assets/Throwable_Objects/BP_Bullet.BP_Bullet_C" (`SceneComponent.K2_GetComponentToWorld` (`self.SpawnPoint`)) "Undefined" "MultiplyWithRoot" null null))))

(fn `Skill`
  (params (Target :type "/Game/HSS/Blueprints/BP_Unit Object Reference"))
  (`PlayerController.SetViewTargetWithBlend` (`GameplayStatics.GetPlayerController` 0) null 0.0 "VTBlend_Linear" 0.0 false))

(fn `UserConstructionScript`
  (`parent.UserConstructionScript`))