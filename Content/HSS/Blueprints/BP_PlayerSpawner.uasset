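; BP_PlayerSpawner is the anchor point for lining up the player units in the turn-based game mode.
; It registers itself with BP_TurnGameMode on BeginPlay.
; RearrangePlayers centers the active player on the spawner and offsets each other valid player to either side by its PlayerIndex difference times PlayerDistance.
; Each moved player then resets its saved original location to match the new position.
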(event `self.ReceiveBeginPlay`
  (bind _asbp_turn_game_mode (cast `/Game/HSS/Blueprints/BP_TurnGameMode` (`GameplayStatics.GetGameMode`))
    (:`then`
      (set `/Game/HSS/Blueprints/BP_TurnGameMode.PlayerSpawner` self _asbp_turn_game_mode))
    (:`CastFailed`
      (`KismetSystemLibrary.PrintString` "CAST FAILED! ! !" true true (struct :`R` 1.0 :`A` 1.0) 30.0))))

(fn `RearrangePlayers`
  (bind _asbp_turn_game_mode (cast `/Game/HSS/Blueprints/BP_TurnGameMode` (`GameplayStatics.GetGameMode`)))
  (bind _asbp_player (cast `/Game/HSS/Blueprints/BP_Player` (`/Game/HSS/Blueprints/BP_TurnGameMode.ActiveUnit` _asbp_turn_game_mode)))
  ; 1. 플레이어 배열을 돌면서 유효한지 확인
  (for _array_element (`/Game/HSS/Blueprints/BP_TurnGameMode.Players` _asbp_turn_game_mode)
    (`/Engine/EditorBlueprintResources/StandardMacros.IsValid` _array_element
      (:`Is Valid`
        ; 2. 턴 플레이어를 스포너 중심으로 두고 순서대로 양 옆에 배치
        (`self.K2_SetActorLocation` _array_element (+ (`self.K2_GetActorLocation`) (* (`self.PlayerDistance`) (- (`/Game/HSS/Blueprints/BP_Player.PlayerIndex` _array_element) (`/Game/HSS/Blueprints/BP_Player.PlayerIndex` _asbp_player)))) false false)
        ; 3. 위치가 바뀌었으니 위치 저장 변수 초기화
        (`/Game/HSS/Blueprints/BP_Player.C_Original_Location` _array_element)))))

(fn `UserConstructionScript`)